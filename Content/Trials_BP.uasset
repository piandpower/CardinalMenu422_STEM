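; Trial prototype for a VR visual-vestibular heading experiment, with conflict and no-conflict trial events that randomly run a standard or comparison movement.
; Movements set SceneRoot location from HMD position, usually scaled by sine/cosine of stored angles; comparisons roll X and Y angles separately.
; Enter separately tests drawing angles without replacement, printing the pick and its endpoint.
; UserInput, ResetOrigin and TrajectoryDisplacement are empty stubs; timeline and DoOnce leftovers are unwired.
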(event Custom|VisualControlTrue
  (bind _deviceposition (Class|HeadMountedDisplayFunctionLibrary|GetOrientationandPosition))
  ;[1 1 1] No Conflict
  ;;[1 1 1] TrueStandard: Move Forward Visual Matches Vestibular
  (Transformation|SetWorldLocation (Variables|Default|GetSceneRoot) (Math|Vector|MakeVector (.x _deviceposition) (.y _deviceposition) 0.0) false false)
  (Utilities|FlowControl|Delay 2.0))

(event Custom|Single%20Trial%20Conflict
  ;[1 1 1] Single Trial Conflict
  (if (Math|Random|RandomBool)
    (CallFunction|VisualControlConflict)
    (else
      (CallFunction|ComparisonTrueCopy))))

(event Custom|VisualControlConflict
  (bind _deviceposition (Class|HeadMountedDisplayFunctionLibrary|GetOrientationandPosition))
  (bind _standardvestibularangles (Variables|Default|GetStandardVestibularAngles))
  (bind _output (Utilities|Array|Get(acopy) _standardvestibularangles))
  ;[1 1 1] Conflict
  ;;[1 1 1] SkewedStandard: Incongruence Visual and Vestibular
  (Transformation|SetWorldLocation (Variables|Default|GetSceneRoot) (Math|Vector|MakeVector (* (Math|Trig|Sin(Degrees) _output) (.x _deviceposition)) (* (Math|Trig|Cos(Degrees) _output) (.y _deviceposition)) 0.0) false false)
  (Utilities|FlowControl|Delay 2.0))

(event Custom|ComparisonTrue
  (bind _returnvalue (Math|Random|RandomIntegerinRange 0 3))
  (bind _deviceposition (Class|HeadMountedDisplayFunctionLibrary|GetOrientationandPosition))
  (bind _trajectorytrialsangles (Variables|Default|GetTrajectoryTrialsAngles))
  (bind _output (Utilities|Array|Get(acopy) _trajectorytrialsangles _returnvalue))
  ;[1 1 1] No Conflict
  ;;[1 1 1] ComparisonTrue
  (Transformation|SetWorldLocation (Variables|Default|GetSceneRoot) (Math|Vector|MakeVector (* (Math|Trig|Sin(Degrees) _output) (.x _deviceposition)) (* (Math|Trig|Cos(Degrees) _output) (.y _deviceposition)) 0.0) false false)
  (CallFunction|UserInput)
  (Utilities|FlowControl|Delay 5.0)
  (CallFunction|ResetOrigin))

(event Custom|Single%20Trial%20No%20Conflict
  ;[1 1 1] Single Trial No Conflict
  (if (Math|Random|RandomBool)
    (CallFunction|VisualControlTrue)
    (else
      (CallFunction|ComparisonTrue))))

(event Custom|ComparisonTrueCopy
  (bind _deviceposition (Class|HeadMountedDisplayFunctionLibrary|GetOrientationandPosition))
  (bind _returnvalue (Math|Random|RandomIntegerinRange 0 3))
  (bind _trajectorytrialsangles (Variables|Default|GetTrajectoryTrialsAngles))
  (bind _output (Utilities|Array|Get(acopy) _trajectorytrialsangles _returnvalue))
  ;[1 1 1] Conflict
  ;;[1 1 1] ComparisonTrue
  (Transformation|SetWorldLocation (Variables|Default|GetSceneRoot) (Math|Vector|MakeVector (* (Math|Trig|Sin(Degrees) _output) (.x _deviceposition)) (* (Math|Trig|Cos(Degrees) _output) (.y _deviceposition)) 0.0) false false)
  (CallFunction|UserInput)
  (Utilities|FlowControl|Delay 5.0)
  (CallFunction|ResetOrigin))

(event Input|KeyboardEvents|Enter
  (params (Key :type Key%20Structure))
  (bind _trajectorywithoutreplacement (Variables|Default|GetTrajectoryWithoutReplacement))
  ;[1 1 1] Without Replacement
  (:Pressed
    (bind _output_get (Variables|Default|SetRandomInteger (Math|Random|RandomIntegerinRange 0 3)))
    (bind _output_get_2 (Variables|Default|SetTrajectoryTrial_WOR (Utilities|Array|Get(acopy) _trajectorywithoutreplacement _output_get)))
    (Development|PrintString (Utilities|String|ToString(Float) _output_get_2))
    (for _array_element (Variables|Default|GetTrajectoryTrialsAngles)
      (if (== _array_element (Variables|Default|GetTrajectoryTrial_WOR))
        (bind _returnvalue (Utilities|Array|RemoveItem _trajectorywithoutreplacement (Variables|Default|GetTrajectoryTrial_WOR)))
        (Development|PrintString (Utilities|String|ToString(Boolean) _returnvalue))
        (else
          (Development|PrintString (Utilities|String|ToString(Boolean) (== _array_element (Variables|Default|GetTrajectoryTrial_WOR))) true true "(R=1.000000,G=0.660000,B=1.000000,A=1.000000)" 0.1)))))
  (:Released
    (if (not (== (Variables|Default|GetTrajectoryTrial_WOR) 0.0))
      (Development|PrintString (Utilities|String|ToString(Float) (Variables|Default|GetTrajectoryTrial_WOR)) true true "(R=0.000000,G=0.000000,B=1.000000,A=1.000000)")
      (Development|PrintString (Utilities|String|Append "Trajectory EndPoint = " (Utilities|String|ToString(Vector2d) (Math|Vector2D|MakeVector2D (* (Math|Trig|Cos(Degrees) (Variables|Default|GetTrajectoryTrial_WOR)) 8.0) (* (Math|Trig|Sin(Degrees) (Variables|Default|GetTrajectoryTrial_WOR)) 8.0)))) true true "(R=0.000000,G=0.000000,B=1.000000,A=1.000000)"))))

(fn ConstructionScript)

(fn ResetOrigin)

(fn UserInput)

(fn TrajectoryDisplacement)